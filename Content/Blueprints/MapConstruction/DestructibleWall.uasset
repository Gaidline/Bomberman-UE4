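; Destructible wall map piece that can drop a random pickup when it is destroyed.
; The Destroy function destroys the actor and returns true.
; The Destroyed event rolls SpawnPickupChance through PickItemByProbability and, on success, spawns a random class from AvailablePickupsToSpawn at the wall's location.
; The construction script only calls the parent's version.
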(event EventDestroyed
  (bind _available_pickups_to_spawn (Variables|Default|GetAvailable%20Pickups%20To%20Spawn))
  (bind _is_picked (CallFunction|PickItembyProbability (Variables|Default|GetSpawn%20Pickup%20Chance)))
  (if _is_picked
    (Game|SpawnActorfromClass (Utilities|Array|Get(acopy) _available_pickups_to_spawn (Math|Random|RandomIntegerinRange 0 (- (Utilities|Array|Length _available_pickups_to_spawn) 1))) (Math|Transform|MakeTransform (Transformation|GetActorLocation) "0, 0, 0" "1,1,1") "Undefined" 0 0)))

(fn ConstructionScript
  (|CallParentFunction))

(fn Destroy
  (Actor|DestroyActor)
  (return true))