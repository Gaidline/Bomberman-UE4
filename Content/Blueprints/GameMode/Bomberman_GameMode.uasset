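; Bomberman game mode that spawns players and decides when a match ends in victory or draw.
; On PostLogin it maps tagged PlayerStarts, then spawns and possesses a Bomberman at one of four starts chosen by player count.
; A looping timer counts controlled Bombermen, triggering Victory for a lone survivor or Draw when none remain or time expires.
; The countdown timer's setup is disconnected, so UpdateGameTime is never started here.
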(event Custom|Update%20Game%20Time
  (bind _bomberman_game_state (Variables|Default|GetBomberman%20Game%20State))
  ;[1 1 1] Update Game countdown
  (Variables|/Game/Blueprints/GameMode/Bomberman_GameState.Bomberman_GameState_C|SetGame%20Time%20Countdown _bomberman_game_state (Math|Float|Clamp(Float) (- (Variables|/Game/Blueprints/GameMode/Bomberman_GameState.Bomberman_GameState_C|GetGame%20Time%20Countdown _bomberman_game_state) 0.1) 0.0 2e+02)))

(event Custom|Validate%20Players
  ;[1 1 1] Check if there are valid Players in game and handle game conditions
  (bind (_num_players_in_game _num_players_logged _last_valid_bomberman) (CallFunction|CountPlayersinGame))
  (Utilities|FlowControl|Sequence
    (:then_0
      (if (>= _num_players_in_game 2)
        (Variables|Default|SetPlaying%20Valid%20Game true)))
    (:then_1
      (if (or (<= _num_players_in_game 0) (and (>= _num_players_in_game 2) (== (Variables|/Game/Blueprints/GameMode/Bomberman_GameState.Bomberman_GameState_C|GetGame%20Time%20Countdown (Variables|Default|GetBomberman%20Game%20State)) 0.0)))
        (Utilities|Time|ClearandInvalidateTimerbyHandle (Variables|Default|GetUpdate%20Game%20Timer))
        (for _array_element (Variables|Default|GetList%20Of%20Players%20%28By%20Controllers%29)
          (bind _asbomberman (Utilities|Casting|CastToBomberman (Pawn|GetControlledPawn _array_element))
            (:then
              (Default|Draw _asbomberman))
            (:CastFailed
              (bind _asspectator (Utilities|Casting|CastToSpectator (Pawn|GetControlledPawn _array_element)))
              (Default|Draw _asspectator))))))
    (:then_2
      (if (and (== _num_players_in_game 1) (Variables|Default|GetPlaying%20Valid%20Game))
        (Utilities|Time|ClearandInvalidateTimerbyHandle (Variables|Default|GetValidate%20Players%20Timer))
        (Utilities|Time|ClearandInvalidateTimerbyHandle (Variables|Default|GetUpdate%20Game%20Timer))
        (Default|Victory _last_valid_bomberman)))))

(event Custom|RespawnPlayerEvent
  (params (PlayerController :type Player%20Controller%20Object%20Reference))
  (bind _returnvalue (Pawn|GetControlledPawn PlayerController))
  ;[1 1 1] Respawns the player at player start location
  (Utilities|IsValid _returnvalue
    (:Is%20Valid
      (Actor|DestroyActor _returnvalue))
    (:Is%20Not%20Valid
      _))
  (switch int (Utilities|Array|Length (Variables|/Script/Engine.GameState|GetPlayerArray (Game|GetGameState)))
    (:1
      (bind _returnvalue_2 (Game|SpawnActorfromClass "/Game/Blueprints/Player/Bomberman.Bomberman_C" (Transformation|GetActorTransform (Variables|Default|GetPlayer%20Start%201)) "AdjustIfPossibleButDontSpawnIfColliding" 0 0))
      (bind _output_get (Variables|Default|SetLast%20Spawned%20Bomberman _returnvalue_2))
      (Pawn|Possess PlayerController _output_get))
    (:2
      (bind _returnvalue_3 (Game|SpawnActorfromClass "/Game/Blueprints/Player/Bomberman.Bomberman_C" (Transformation|GetActorTransform (Variables|Default|GetPlayer%20Start%202)) "AdjustIfPossibleButDontSpawnIfColliding" 0 0))
      (bind _output_get_2 (Variables|Default|SetLast%20Spawned%20Bomberman _returnvalue_3))
      (Pawn|Possess PlayerController _output_get_2))
    (:3
      (bind _returnvalue_4 (Game|SpawnActorfromClass "/Game/Blueprints/Player/Bomberman.Bomberman_C" (Transformation|GetActorTransform (Variables|Default|GetPlayer%20Start%203)) "AdjustIfPossibleButDontSpawnIfColliding" 0 0))
      (bind _output_get_3 (Variables|Default|SetLast%20Spawned%20Bomberman _returnvalue_4))
      (Pawn|Possess PlayerController _output_get_3))
    (:4
      (bind _returnvalue_5 (Game|SpawnActorfromClass "/Game/Blueprints/Player/Bomberman.Bomberman_C" (Transformation|GetActorTransform (Variables|Default|GetPlayer%20Start%204)) "AdjustIfPossibleButDontSpawnIfColliding" 0 0))
      (bind _output_get_4 (Variables|Default|SetLast%20Spawned%20Bomberman _returnvalue_5))
      (Pawn|Possess PlayerController _output_get_4)))
  (bind _asbomberman_game_instance (Utilities|Casting|CastToBomberman_GameInstance (Game|GetGameInstance)))
  (Variables|/Game/Blueprints/GameMode/Bomberman_GameInstance.Bomberman_GameInstance_C|SetLocal%20Player%20Id _asbomberman_game_instance (Variables|/Script/Engine.PlayerState|GetPlayerId (Variables|/Script/Engine.Controller|GetPlayerState PlayerController)))
  (Utilities|Array|Add (Variables|Default|GetList%20Of%20Players%20%28By%20Controllers%29) PlayerController)
  (Utilities|FlowControl|Delay 0.5) ; Wait for Posses to complete
  (Default|SetupViewTarget (Variables|Default|GetLast%20Spawned%20Bomberman))
  (Default|CallOnBombermanSpawned (Variables|Default|GetLast%20Spawned%20Bomberman)))

(event EventBeginPlay
  ;[0.02154 0.825 0.05275] Begin
  (Utilities|FlowControl|Sequence
    (:then_0
      (bind _returnvalue (Utilities|Time|SetTimerbyFunctionName 0 "Validate Players" 1.5 true))
      (Variables|Default|SetValidate%20Players%20Timer _returnvalue)
      (bind _asbomberman_game_state (Utilities|Casting|CastToBomberman_GameState (Game|GetGameState)))
      (Variables|Default|SetBomberman%20Game%20State _asbomberman_game_state))
    (:then_1
      (Variables|/Game/Blueprints/GameMode/Bomberman_GameState.Bomberman_GameState_C|SetGame%20Time%20Countdown (Variables|Default|GetBomberman%20Game%20State) 6e+01))))

(event EventPostLogin
  (params (NewPlayer :type Player%20Controller%20Object%20Reference))
  ;[1 1 1] Post login
  (Networking|SwitchHasAuthority
    (:Authority
      (bind _outactors (Actor|GetAllActorsOfClass "/Script/Engine.PlayerStart"))
      (for _array_element _outactors
        (switch name (Variables|/Script/Engine.PlayerStart|GetPlayerStartTag _array_element)
          (:Player%201
            (Variables|Default|SetPlayer%20Start%201 _array_element))
          (:Player%202
            (Variables|Default|SetPlayer%20Start%202 _array_element))
          (:Player%203
            (Variables|Default|SetPlayer%20Start%203 _array_element))
          (:Player%204
            (Variables|Default|SetPlayer%20Start%204 _array_element))))
      (CallFunction|RespawnPlayerEvent NewPlayer))))

(fn ConstructionScript)

(fn CountPlayersinGame
  (for _array_element (Variables|Default|GetList%20Of%20Players%20%28By%20Controllers%29)
    (Utilities|IsValid _array_element
      (:Is%20Valid
        (Math|Integer|IncrementInt (LocalVariables|Get_Num%20Players%20Logged)
          (:%20%20
            (bind _asbomberman (Utilities|Casting|CastToBomberman (Pawn|GetControlledPawn _array_element)))
            (Math|Integer|IncrementInt (LocalVariables|Get_Num%20Players%20In%20Game)
              (:%20%20
                (LocalVariables|Set_Last%20Valid%20Bomberman _asbomberman))))))))
  (return (LocalVariables|Get_Num%20Players%20In%20Game) (LocalVariables|Get_Num%20Players%20Logged) (LocalVariables|Get_Last%20Valid%20Bomberman)))