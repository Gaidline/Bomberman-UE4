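; Base player class for a Bomberman game, handling camera setup, match-draw feedback and quitting.
; It points its controller's view at the main camera held by the GameState.
; A draw fires once, using client RPCs to replace any previous message dialog and pause the game.
; The Exit input has the authority destroy the session through the GameInstance, then quits the game.
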(event Custom|Setup%20View%20Target
  ;[1 1 1] Change View Target to Main Camera
  (bind _asbomberman_game_state (Utilities|Casting|CastToBomberman_GameState (Game|GetGameState)))
  (bind _asplayer_controller (Utilities|Casting|CastToPlayerController (Pawn|GetController)))
  (Utilities|IsValid (Default|GetMainCamera _asbomberman_game_state)
    (:Is%20Valid
      (Game|Player|SetViewTargetwithBlend _asplayer_controller (Default|GetMainCamera _asbomberman_game_state) 0.0 "VTBlend_Linear" 0.0 false))))

(event Custom|Show%20Message%20Dialog%20%28Client%29
  (params (Message :type String))
  ;[1 1 1] Show message dialog for the right Player
  (bind _last_message_dialog (Variables|Default|GetLast%20Message%20Dialog)
    (:then
      (Widget|RemovefromParent _last_message_dialog))
    (:else
      _))
  (bind _returnvalue (UserInterface|CreateWidget "/Game/Blueprints/HUD/MessageDialog.MessageDialog_C" 0 Message))
  (bind _output_get (Variables|Default|SetLast%20Message%20Dialog _returnvalue))
  (UserInterface|Viewport|AddtoViewport _output_get 0))

(event Custom|Pause%20Game%20%28Client%29
  ;[1 1 1] Pause game
  (bind _returnvalue (Game|SetGamePaused true))
  (Development|PrintString (Utilities|String|ToString(Boolean) _returnvalue) true true "(R=0.000000,G=0.660000,B=1.000000,A=1.000000)" 5.0))

(event Custom|Draw
  ;[1 1 1] On Players draw
  (Utilities|FlowControl|DoOnce false
    (:Completed
      (CallFunction|ShowMessageDialog(Client) "Draw")
      (CallFunction|PauseGame(Client)))))

(event Input|ActionEvents|InputActionExit
  (params (Key :type Key%20Structure :default "AnyKey"))
  ;[1 1 1] Exit game
  (:Pressed
    (Utilities|FlowControl|Sequence
      (:then_0
        (Networking|SwitchHasAuthority
          (:Authority
            (bind _asbomberman_game_instance (Utilities|Casting|CastToBomberman_GameInstance (Game|GetGameInstance)))
            (Default|DestroySessionCaller _asbomberman_game_instance))))
      (:then_1
        (Game|QuitGame 0 "Quit")))))

(fn ConstructionScript)