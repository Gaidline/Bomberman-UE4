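; Spectator pawn for the Bomberman multiplayer game, giving a non-playing player the match HUD and a view of the arena.
; On BeginPlay it adds the Bomberman HUD, refreshing its player list on request, and can switch the view target to the GameState's main camera.
; Client RPCs show message dialogs and pause, while a draw shows a message, then has the server destroy the session and open the Lobby.
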(event Custom|Setup%20View%20Target
  ;[1 1 1] Change View Target to Main Camera
  (bind _asbomberman_game_state (Utilities|Casting|CastToBomberman_GameState (Game|GetGameState)))
  (bind _asplayer_controller (Utilities|Casting|CastToPlayerController (Pawn|GetController)))
  (Utilities|IsValid (Default|GetMainCamera _asbomberman_game_state)
    (:Is%20Valid
      (Game|Player|SetViewTargetwithBlend _asplayer_controller (Default|GetMainCamera _asbomberman_game_state) 0.0 "VTBlend_Linear" 0.0 false))))

(event Custom|Destroy%20Session%20%28Server%29
  ;[1 1 1] Request Session destroy by Server
  (bind _asbomberman_game_instance (Utilities|Casting|CastToBomberman_GameInstance (Game|GetGameInstance)))
  (Default|DestroySessionCaller _asbomberman_game_instance)
  (Game|OpenLevel(byName) "Lobby"))

(event Custom|Show%20Message%20Dialog%20%28Client%29
  (params (Message :type String))
  ;[1 1 1] Show message dialog for the right Player
  (bind _bomberman_last_message_dialog (Variables|Default|GetBomberman%20Last%20Message%20Dialog)
    (:then
      (Widget|RemovefromParent _bomberman_last_message_dialog))
    (:else
      _))
  (bind _last_message_dialog (Variables|Default|GetLast%20Message%20Dialog)
    (:then
      (Widget|RemovefromParent _last_message_dialog))
    (:else
      _))
  (bind _returnvalue (UserInterface|CreateWidget "/Game/Blueprints/HUD/MessageDialog.MessageDialog_C" 0 Message))
  (bind _output_get (Variables|Default|SetLast%20Message%20Dialog _returnvalue))
  (UserInterface|Viewport|AddtoViewport _output_get 0))

(event Custom|Update%20Player%20HUD%20List
  ;[1 1 1] Update Player HUD List
  (bind _bomberman_hud (Variables|Default|GetBomberman%20HUD)
    (:then
      (Default|UpdatePlayerList _bomberman_hud))
    (:else)))

(event Custom|Pause%20Game%20%28Client%29
  ;[1 1 1] Pause game
  (Game|SetGamePaused true))

(event Custom|Draw
  ;[1 1 1] On Players draw
  (Utilities|FlowControl|DoOnce false
    (:Completed
      (CallFunction|ShowMessageDialog(Client) "Draw")
      (Utilities|FlowControl|Delay 5.0)
      (CallFunction|DestroySession(Server)))))

(event EventBeginPlay
  ;[1 1 1] Create HUD
  (bind _asplayer_controller (Utilities|Casting|CastToPlayerController (Pawn|GetController)))
  (bind _returnvalue (UserInterface|CreateWidget "/Game/Blueprints/HUD/Bomberman_HUD.Bomberman_HUD_C" _asplayer_controller))
  (bind _output_get (Variables|Default|SetBomberman%20HUD _returnvalue))
  (UserInterface|Viewport|AddtoViewport _output_get 0)
  (Default|UpdatePlayerList _output_get))

(event Input|ActionEvents|InputActionExit
  (params (Key :type Key%20Structure :default "AnyKey"))
  ;[1 1 1] Exit game
  (:Pressed
    (Utilities|FlowControl|Sequence
      (:then_0
        (Networking|SwitchHasAuthority
          (:Authority
            (bind _asbomberman_game_instance (Utilities|Casting|CastToBomberman_GameInstance (Game|GetGameInstance)))
            (Default|DestroySessionCaller _asbomberman_game_instance))))
      (:then_1
        (Game|QuitGame 0 "Quit")))))

(fn ConstructionScript)