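; Bomb actor for a Bomberman-style game that explodes on a timer after being planted.
; On explosion it sphere-traces along the GameState's world forward, backward, right and left axes up to the blast length.
; Each hit actor gets a DestroyMessage, and a false return stops that ray so immortal objects shield what is behind them.
; After a short delay it notifies its instigator and destroys itself.
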(event Custom|Explode
  ;[1 1 1] Explode Bomb
  (Utilities|FlowControl|Sequence
    (:then_0
      (bind _asbomberman_game_state (Utilities|Casting|CastToBomberman_GameState (Game|GetGameState)))
      (Utilities|FlowControl|Sequence
        (:then_0
          (CallFunction|BlastinDirection (Variables|/Game/Blueprints/GameMode/Bomberman_GameState.Bomberman_GameState_C|GetWorld%20Forward _asbomberman_game_state)) ; Forward Blast
        )
        (:then_1
          (CallFunction|BlastinDirection (* (Variables|/Game/Blueprints/GameMode/Bomberman_GameState.Bomberman_GameState_C|GetWorld%20Forward _asbomberman_game_state) -1.0)) ; Backward Blast
        )
        (:then_2
          (CallFunction|BlastinDirection (Variables|/Game/Blueprints/GameMode/Bomberman_GameState.Bomberman_GameState_C|GetWorld%20Right _asbomberman_game_state)) ; Right Blast
        )
        (:then_3
          (CallFunction|BlastinDirection (* (Variables|/Game/Blueprints/GameMode/Bomberman_GameState.Bomberman_GameState_C|GetWorld%20Right _asbomberman_game_state) -1.0)) ; Left Blast
        )))
    (:then_1
      (Utilities|FlowControl|Delay 2.0)
      (Class|BombermanInterface|PlantedBombDestroyed(Message) (Game|GetInstigator))
      (Actor|DestroyActor))))

(event EventBeginPlay
  ;[0.1251 0.88 0.01692] Start Bomb timer
  (Utilities|Time|SetTimerbyFunctionName 0 "Explode" (Variables|Default|GetBomb%20Delay%20Time)))

(fn ConstructionScript)

(fn BlastinDirection
  (params (Direction :type Vector))
  (bind _returnvalue (Transformation|GetActorLocation))
  (bind _outhits (Collision|MultiSphereTraceForObjects _returnvalue (+ _returnvalue (* Direction (Variables|Default|GetBlast%20Length))) 5e+01 (Utilities|Array|MakeArray "ObjectTypeQuery6" "ObjectTypeQuery8" "ObjectTypeQuery7" "ObjectTypeQuery3") false 0 "ForDuration"))
  (bind _array_element (Utilities|Array|ForEachLoopwithBreak _outhits :!label _label)
    (:LoopBody
      (bind _success (Class|WeaponInteractInterface|Destroy(Message) (.HitActor (Collision|BreakHitResult _array_element))))
      (if (not _success) ; If blast meets Immortal object, stop destroying objects behind it
        (goto _label Break)))))